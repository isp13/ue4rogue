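; BP_EnemyProjectile is a projectile fired by enemies in the 2D roguelike kit that damages the player.
; On overlap it destroys itself against rooms and breakables, or applies its Damage to BP_Player and then destroys itself, ignoring other actors.
; SetDirection launches it by setting the ProjectileMovement velocity in local space from a direction vector scaled by Speed.
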(event `self.ReceiveActorBeginOverlap`
  (params (OtherActor :type "Actor Object Reference"))
  ;[1 1 1] Destroy projectile on overlap Room or Breakable
  (cast `/Game/Roguelike2DKit/Blueprints/Rooms/BP_BaseRoom` OtherActor
    (:`then`
      (`/Engine/EditorBlueprintResources/StandardMacros.IsValid` self :!label _label
        (:`Is Valid`
          (`self.K2_DestroyActor`))))
    (:`CastFailed`
      (cast `/Game/Roguelike2DKit/Blueprints/Terrain/BP_BaseBreakable` OtherActor
        (:`then`
          (goto _label))
        (:`CastFailed`
          ;[1 1 1] Apply damage to player on overlap and destroy projectile
          (bind _asbp_player (cast `/Game/Roguelike2DKit/Blueprints/Characters/Player/BP_Player` OtherActor))
          (`GameplayStatics.ApplyDamage` _asbp_player (`self.Damage`))
          (`self.K2_DestroyActor`))))))

(fn `SetDirection`
  (params (DirectionVector :type "Vector Structure"))
  ;[1 1 1] Set velocity of projectile using direction vector and speed
  (`ProjectileMovementComponent.SetVelocityInLocalSpace` (`self.ProjectileMovement`) (* DirectionVector (`self.Speed`))))

(fn `UserConstructionScript`)