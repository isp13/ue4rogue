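; BP_PlayerProjectile is the player's projectile in the roguelike 2D kit, damaging enemies it hits.
; SetDirection converts a direction to a vector, scales it by Speed and sets it as the ProjectileMovement component's local-space velocity.
; On actor overlap, rooms and breakables only destroy the projectile, while enemies receive Damage through ApplyDamage before it is destroyed.
; Overlaps with any other actor are ignored.
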(event `self.ReceiveActorBeginOverlap`
  (params (OtherActor :type "Actor Object Reference"))
  ;[1 1 1] Destroy projectile on overlap Room or Breakable
  (cast `/Game/Roguelike2DKit/Blueprints/Rooms/BP_BaseRoom` OtherActor
    (:`then`
      (`/Engine/EditorBlueprintResources/StandardMacros.IsValid` self :!label _label
        (:`Is Valid`
          (`self.K2_DestroyActor`))))
    (:`CastFailed`
      (cast `/Game/Roguelike2DKit/Blueprints/Terrain/BP_BaseBreakable` OtherActor
        (:`then`
          (goto _label))
        (:`CastFailed`
          ;[1 1 1] Apply damage to enemy on overlap and destroy projectile
          (bind _asbp_enemy (cast `/Game/Roguelike2DKit/Blueprints/Characters/Enemies/BP_Enemy` OtherActor))
          (`GameplayStatics.ApplyDamage` _asbp_enemy (`self.Damage`))
          (`self.K2_DestroyActor`))))))

(fn `SetDirection`
  (params (Direction :type "/Game/Roguelike2DKit/Blueprints/Directions/ENUM_Directions Enum" :default "NewEnumerator4"))
  ;[1 1 1] Set velocity of projectile using direction vector and speed
  (`ProjectileMovementComponent.SetVelocityInLocalSpace` (`self.ProjectileMovement`) (* (`/Game/Roguelike2DKit/Blueprints/Directions/BP_DirectionFunctionLibrary.DirectionToVector` Direction) (`self.Speed`))))

(fn `UserConstructionScript`)