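; Powerup pickup actor that applies its powerups to the player on pickup, plays its sound and destroys itself.
; The construction script picks a random value from the powerup name enum.
; That name is used as the row key into DT_PowerupItems, which supplies the sprite, color, pickup sound and powerups, printing an error if the row is missing.
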(event `/Game/Roguelike2DKit/Blueprints/Pickups/BP_iPickup.OnPickup`
  (params (Player :type "/Game/Roguelike2DKit/Blueprints/Characters/Player/BP_Player Object Reference"))
  ;[1 1 1] Apply Powerups to player, play sound and destroy itself
  (`/Game/Roguelike2DKit/Blueprints/Characters/Player/BP_Player.ApplyPowerups` Player (`self.Powerups`))
  (`GameplayStatics.PlaySound2D` (`self.PickupSound`))
  (`self.K2_DestroyActor`))

(fn `LoadPowerupProperties`
  ;[1 1 1] Get options and powerups from DataTable using Powerup Name (enum) value
  (bind _returnvalue (`|GetDataTableRow` "/Game/Roguelike2DKit/Blueprints/Powerups/DT_PowerupItems.DT_PowerupItems" (`KismetStringLibrary.Conv_StringToName` (`|GetEnumeratorNameAsString` (`self.PowerupName`))))
    (:`then`
      (`|ExecutionSequence`
        (:`then_0`
          (bind (_name _sprite _color _pickupsound _powerups) (break `/Game/Roguelike2DKit/Blueprints/Powerups/STR_PowerupItem` _returnvalue))
          ;[1 1 1] Set sprite
          (`PaperSpriteComponent.SetSprite` (`self.Sprite`) _sprite))
        (:`then_1`
          ;[1 1 1] Set sprite color
          (`PaperSpriteComponent.SetSpriteColor` (`self.Sprite`) _color))
        (:`then_2`
          ;[1 1 1] Set pickup sound
          (set `self.PickupSound` _pickupsound))
        (:`then_3`
          ;[1 1 1] Set powerups
          (set `self.Powerups` _powerups))))
    (:`RowNotFound`
      ;[1 1 1] Print error for invalid PowerupName
      (`KismetSystemLibrary.PrintString` "PowerupName not found in DataTable"))))

(fn `RandomPowerupName`
  (returns (PowerupName :type "/Game/Roguelike2DKit/Blueprints/Powerups/ENUM_PowerupNames Enum"))
  (return (cast `/Game/Roguelike2DKit/Blueprints/Powerups/ENUM_PowerupNames` (`KismetMathLibrary.Conv_IntToByte` (`KismetMathLibrary.RandomIntegerInRange` 0 (- (enumcount `/Game/Roguelike2DKit/Blueprints/Powerups/ENUM_PowerupNames`) 1))))))

(fn `SetRandomType`
  ;[1 1 1] Set powerup name
  (set `self.PowerupName` (`self.RandomPowerupName`))
  ;[1 1 1] Load powerup properties from DataTable
  (`self.LoadPowerupProperties`))

(fn `UserConstructionScript`
  (`parent.UserConstructionScript`)
  ;[1 1 1] Set pickup to random Powerup
  (`self.SetRandomType`))