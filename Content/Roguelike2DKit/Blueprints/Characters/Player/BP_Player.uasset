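; Player character for a 2D roguelike that moves, shoots in four directions, drops bombs, carries keys and triggers game over on death.
; Tick applies swept movement with wall sliding and turns shoot input into a looping fire timer, paused on release to preserve the fire-rate delay.
; Powerups adjust clamped levels that recompute health, damage, speed, fire rate and range.
; Damage routes through BPHealthComponent, and GodMode ignores it and boosts projectile damage.
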(event `self.ReceiveBeginPlay`
  ;[1 1 1] Save the game mode in a variable for future use
  (bind _asbp_roguelike_2dgame_mode (cast `/Game/Roguelike2DKit/Blueprints/Game/BP_Roguelike2DGameMode` (`GameplayStatics.GetGameMode`)))
  (set `self.GameMode` _asbp_roguelike_2dgame_mode)
  ;[1 1 1] Initialize Health Component
  (`/Game/Roguelike2DKit/Blueprints/Characters/BP_HealthComponent.InitializeHealth` (`self.BP_HealthComponent`)))

(event `InputAction|PlaceBomb`
  (params (Key :type "Key Structure"))
  ;[1 1 1] Place bombs
  (:`Pressed`
    (`self.SpawnBomb`)))

(event `self.ReceiveAnyDamage`
  (params (Damage :type "Float (single-precision)") (DamageType :type "DamageType Object Reference") (InstigatedBy :type "Controller Object Reference") (DamageCauser :type "Actor Object Reference"))
  ;[1 1 1] Handle damage on event AnyDamage
  (`self.HandleDamage` Damage))

(event `self.ReceiveTick`
  (params (DeltaSeconds :type "Float (single-precision)"))
  ;[1 1 1] Update movement and shooting, if not game over
  (bind _gamemode (`self.GameMode`)
    (:`then`
      (if (not (`/Game/Roguelike2DKit/Blueprints/Game/BP_Roguelike2DGameMode.IsGameOver` _gamemode))
        (`self.UpdateMovement` DeltaSeconds)
        (`self.UpdateShooting`)))
    (:`else`)))

(event `UpdateMovement`
  (params (DeltaSeconds :type "Float (double-precision)"))
  ;[1 1 1] Handle movement and shoot input
  (`self.ApplyMovementInput` DeltaSeconds))

(event `UpdateShooting`
  ;[1 1 1] Handle movement and shoot input
  (`self.HandleShootInput` (`self.GetInputAxisValue`) (`self.GetInputAxisValue`)))

(event `HandleShootInput`
  (params (ShootUp :type "Float (double-precision)") (ShootRight :type "Float (double-precision)"))
  (bind _firetimer (`self.FireTimer`))
  ;[1 1 1] Update direction based on input
  (bind _output_get (set `self.FireDirection` (`self.GetFireDirection` ShootUp ShootRight)))
  (switch `/Game/Roguelike2DKit/Blueprints/Directions/ENUM_Directions` _output_get
    (:`NewEnumerator4`
      ;[1 1 1] Pause firing without input
      (if (and (`KismetSystemLibrary.K2_IsValidTimerHandle` _firetimer) (`KismetSystemLibrary.K2_IsTimerActiveHandle` _firetimer))
        (`KismetSystemLibrary.K2_PauseTimerHandle` (`self.FireTimer`))
        ;[1 1 1] After the remaining fire rate delay, stop the timer unless it has become active again
        (`KismetSystemLibrary.Delay` (`KismetSystemLibrary.K2_GetTimerRemainingTimeHandle` (`self.FireTimer`)))
        (if (`KismetSystemLibrary.K2_IsTimerPausedHandle` (`self.FireTimer`))
          (`self.StopFiring`))))
    (:`NewEnumerator0`
      ;[1 1 1] Start firing unless the timer is already active
      (if (or (`KismetSystemLibrary.K2_IsValidTimerHandle` (`self.FireTimer`)) (not (`KismetSystemLibrary.K2_IsTimerActiveHandle` (`self.FireTimer`)))) :!label _label
        (`self.StartFiring` (`self.FireDirection`))))
    (:`NewEnumerator1`
      (goto _label))
    (:`NewEnumerator2`
      (goto _label))
    (:`NewEnumerator3`
      (goto _label))))

(fn `AddBombs`
  (params (Delta :type Integer))
  ;[1 1 1] Add delta amount to bombs
  (set `self.Bombs` (+ Delta (`self.Bombs`))))

(fn `AddKeys`
  (params (Delta :type Integer))
  ;[1 1 1] Add delta amount to keys
  (set `self.Keys` (+ Delta (`self.Keys`))))

(fn `ApplyMovementInput`
  (params (DeltaTime :type "Float (double-precision)"))
  (locals (Offset :type "Float (double-precision)") (InputDirection :type "Vector Structure" :default (0.0 0.0 0.0)))
  ;[1 1 1] Determine move offset for this frame
  (set `local.Offset` (* DeltaTime (`self.MovementSpeed`)))
  ;[1 1 1] Determine input direction
  (set `local.InputDirection` (`KismetMathLibrary.Normal` (`KismetMathLibrary.MakeVector` (`self.GetInputAxisValue`) 0.0 (`self.GetInputAxisValue`))))
  ;[1 1 1] Apply the offset to the actor
  (bind _sweephitresult (`self.K2_AddActorWorldOffset` (* (`local.InputDirection`) (`local.Offset`)) true))
  (bind (_bblockinghit _binitialoverlap _time _distance _location _impactpoint _normal) (`GameplayStatics.BreakHitResult` _sweephitresult))
  ;[1 1 1] Check if it's a blocking hit (e.g. walk into wall)
  (if _bblockinghit
    ;[1 1 1] Apply the offset in the new direction
    (`self.K2_AddActorWorldOffset` (* (`KismetMathLibrary.Normal` (- (`local.InputDirection`) (* _normal (`KismetMathLibrary.Dot_VectorVector` (`local.InputDirection`) _normal)))) (`local.Offset`)) true)))

(fn `ApplyPowerups`
  (params (Upgrades :type "Array of /Game/Roguelike2DKit/Blueprints/Powerups/STR_Powerup Structure"))
  (locals (LevelDelta :type Integer))
  ;[1 1 1] Loop over powerups
  (for _array_element Upgrades
    (bind (_power _leveldelta) (break `/Game/Roguelike2DKit/Blueprints/Powerups/STR_Powerup` _array_element))
    ;[1 1 1] Switch on power type
    (set `local.LevelDelta` _leveldelta)
    (switch `/Game/Roguelike2DKit/Blueprints/Powerups/ENUM_Powers` _power
      (:`NewEnumerator0`
        ;[1 1 1] Apply powerup with level delta
        (`self.PowerupMaxHealth` (`local.LevelDelta`)))
      (:`NewEnumerator1`
        (`self.PowerupDamage` (`local.LevelDelta`)))
      (:`NewEnumerator2`
        (`self.PowerupMovementSpeed` (`local.LevelDelta`)))
      (:`NewEnumerator3`
        (`self.PowerupFireRate` (`local.LevelDelta`)))
      (:`NewEnumerator4`
        (`self.PowerupFireRange` (`local.LevelDelta`))))))

(fn `FireProjectile`
  (locals (Projectile :type "/Game/Roguelike2DKit/Blueprints/Projectiles/BP_PlayerProjectile Object Reference"))
  ;[1 1 1] Spawn projectile based on player location and offset and set the projectile scale
  (bind _returnvalue (`|SpawnActorFromClass` "/Game/Roguelike2DKit/Blueprints/Projectiles/BP_PlayerProjectile.BP_PlayerProjectile_C" (`KismetMathLibrary.MakeTransform` (+ (`self.K2_GetActorLocation`) (* (`/Game/Roguelike2DKit/Blueprints/Directions/BP_DirectionFunctionLibrary.DirectionToVector` (`self.FireDirection`)) (`self.ProjectileSpawnOffset`))) (struct) (`self.ProjectileScale`)) "Undefined" "OverrideRootScale" null null))
  (bind _output_get (set `local.Projectile` _returnvalue))
  (`/Engine/EditorBlueprintResources/StandardMacros.IsValid` _output_get
    (:`Is Valid`
      (`|ExecutionSequence`
        (:`then_0`
          ;[1 1 1] Set projectile damage (999 if god mode)
          (set `/Game/Roguelike2DKit/Blueprints/Projectiles/BP_PlayerProjectile.Damage` (select `bool` (`self.GodMode`) :`false` (`self.ProjectileDamage`) :`true` 999.0) (`local.Projectile`)))
        (:`then_1`
          ;[1 1 1] Set fire range (projectile life span)
          (`self.SetLifeSpan` (`local.Projectile`) (`self.Fire Range`)))
        (:`then_2`
          ;[1 1 1] Set projectile direction
          (`/Game/Roguelike2DKit/Blueprints/Projectiles/BP_PlayerProjectile.SetDirection` (`local.Projectile`) (`self.FireDirection`)))))))

(fn `GetFireDirection`
  (params (ShootUp :type "Float (double-precision)") (ShootRight :type "Float (double-precision)"))
  (returns (Direction :type "/Game/Roguelike2DKit/Blueprints/Directions/ENUM_Directions Enum"))
  (locals (Result :type "/Game/Roguelike2DKit/Blueprints/Directions/ENUM_Directions Enum"))
  ;[1 1 1] Return North, South, East, West or None based on fire input
  (if (> ShootUp (`self.FireInputThreshold`))
    (set `local.Result` "NewEnumerator0")
    (elif (< ShootUp (* (`self.FireInputThreshold`) -1.0))
      (set `local.Result` "NewEnumerator1")
      (elif (> ShootRight (`self.FireInputThreshold`))
        (set `local.Result` "NewEnumerator2")
        (elif (< ShootRight (* (`self.FireInputThreshold`) -1.0))
          (set `local.Result` "NewEnumerator3")
          (else
            (set `local.Result` "NewEnumerator4"))))))
  (return (`local.Result`)))

(fn `HandleDamage`
  (params (DamageAmount :type "Float (double-precision)"))
  ;[1 1 1] Check god mode. If enabled, ignore the damage
  (if (not (`self.GodMode`))
    (`|ExecutionSequence`
      (:`then_0`
        ;[1 1 1] Play sound
        (`GameplayStatics.PlaySound2D` (`self.PlayerHitSound`)))
      (:`then_1`
        ;[1 1 1] Handle Damage in Component
        (bind _died (`/Game/Roguelike2DKit/Blueprints/Characters/BP_HealthComponent.OnDamage` (`self.BP_HealthComponent`) DamageAmount))
        ;[1 1 1] If dead, handle Death
        (if _died
          (`self.HandleDeath`))))))

(fn `HandleDeath`
  ;[1 1 1] Handle game over in game mode
  (bind _gamemode (`self.GameMode`)
    (:`then`
      (`/Game/Roguelike2DKit/Blueprints/Game/BP_Roguelike2DGameMode.GameOver` _gamemode)
      ;[1 1 1] Stop firing timer
      (`self.StopFiring`)
      ;[1 1 1] Update sprite to dead flipbook
      (`PaperFlipbookComponent.SetFlipbook` (`self.Sprite`) (`self.DeadFlipbook`)))
    (:`else`)))

(fn `HasBombs`
  (returns (HasBombs :type Boolean))
  ;[1 1 1] Returns whether the player has bombs
  (return (> (`self.Bombs`) 0)))

(fn `HasKeys`
  (returns (HasKeys :type Boolean))
  ;[1 1 1] Returns whether the player has keys
  (return (> (`self.Keys`) 0)))

(fn `PowerupDamage`
  (params (`Level delta` :type Integer))
  ;[1 1 1] Increases the projectile damage by delta and clamp between 0 an maximum powerup level
  (bind _output_get (set `self.ProjectileDamageLevel` (`KismetMathLibrary.Clamp` (+ `Level delta` (`self.ProjectileDamageLevel`)) 0 (`self.MaxPowerupLevel`))))
  ;[1 1 1] Set projectile damage based on level (damage per level * level + base)
  (set `self.ProjectileDamage` (+ (* _output_get (`self.ProjectileDamagePerLevel`)) (`self.BaseProjectileDamage`))))

(fn `PowerupFireRange`
  (params (`Level delta` :type Integer))
  ;[1 1 1] Increases the fire rate by delta and clamp between 0 an maximum powerup level
  (bind _output_get (set `self.FireRangeLevel` (`KismetMathLibrary.Clamp` (+ `Level delta` (`self.FireRangeLevel`)) 0 (`self.MaxPowerupLevel`))))
  ;[1 1 1] Set fire range based on level (fire range per level * level + base)
  (set `self.Fire Range` (+ (* _output_get (`self.FireRangePerLevel`)) (`self.BaseFireRange`))))

(fn `PowerupFireRate`
  (params (`Level delta` :type Integer))
  ;[1 1 1] Increases the fire rate by delta and clamp between 0 an maximum powerup level
  (bind _output_get (set `self.FireRateLevel` (`KismetMathLibrary.Clamp` (+ `Level delta` (`self.FireRateLevel`)) 0 (`self.MaxPowerupLevel`))))
  ;[1 1 1] Set fire rate based on level (fire rate per level * level + base)
  (set `self.FireRate` (+ (* _output_get (`self.FireRatePerLevel`)) (`self.BaseFireRate`))))

(fn `PowerupMaxHealth`
  (params (`Level delta` :type Integer))
  ;[1 1 1] Increases the maximum health by delta and clamp between 0 an maximum powerup level
  (bind _output_get (set `self.MaxHealthLevel` (`KismetMathLibrary.Clamp` (+ `Level delta` (`self.MaxHealthLevel`)) 0 (`self.MaxPowerupLevel`))))
  ;[1 1 1] Set maximum health based on level (health per level * level + base)
  (`/Game/Roguelike2DKit/Blueprints/Characters/BP_HealthComponent.ChangeMaxHealth` (`self.BP_HealthComponent`) (+ (* _output_get (`self.MaxHealthPerLevel`)) (`self.BaseMaxHealth`)) false))

(fn `PowerupMovementSpeed`
  (params (`Level delta` :type Integer))
  ;[1 1 1] Increases the movement speed by delta and clamp between 0 an maximum powerup level
  (bind _output_get (set `self.MovementSpeedLevel` (`KismetMathLibrary.Clamp` (+ `Level delta` (`self.MovementSpeedLevel`)) 0 (`self.MaxPowerupLevel`))))
  ;[1 1 1] Set movement speed based on level (movement speed per level * level + base)
  (set `self.MovementSpeed` (+ (* _output_get (`self.MovementSpeedPerLevel`)) (`self.BaseMovementSpeed`))))

(fn `SpawnBomb`
  ;[1 1 1] Check if player has bombs
  (if (`self.HasBombs`)
    ;[1 1 1] Reduce bomb number and spawn bomb
    (`self.AddBombs` -1)
    (`|SpawnActorFromClass` "/Game/Roguelike2DKit/Blueprints/Items/BP_Bomb.BP_Bomb_C" (`self.GetTransform`) "Undefined" "OverrideRootScale" null null)))

(fn `StartFiring`
  (params (Direction :type "/Game/Roguelike2DKit/Blueprints/Directions/ENUM_Directions Enum" :default "NewEnumerator4"))
  ;[1 1 1] Set fire direction
  (set `self.FireDirection` Direction)
  ;[1 1 1] Check not dead or firing
  (if (and (not (`self.Firing`)) (not (`/Game/Roguelike2DKit/Blueprints/Characters/BP_HealthComponent.IsDead` (`self.BP_HealthComponent`))))
    ;[1 1 1] Set firing to true
    (set `self.Firing` true)
    ;[1 1 1] Fire first projectile
    (`self.FireProjectile`)
    ;[1 1 1] Set looping timer for Fire Projectile with 1/FireRate delay
    (bind _returnvalue (`KismetSystemLibrary.K2_SetTimer` null "FireProjectile" (/ 1.0 (`self.FireRate`)) true))
    ;[1 1 1] Save the fire timer
    (set `self.FireTimer` _returnvalue)))

(fn `StopFiring`
  ;[1 1 1] Stop the timer and update Firing
  (`KismetSystemLibrary.K2_ClearAndInvalidateTimerHandle` (`self.FireTimer`))
  (set `self.Firing` false))

(fn `UserConstructionScript`)