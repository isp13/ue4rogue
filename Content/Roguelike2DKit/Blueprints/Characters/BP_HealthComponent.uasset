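; Health component for Roguelike 2D Kit characters that tracks current and max health, death state and optional regeneration.
; All changes go through ChangeHealth, which clamps the value, updates IsDead and ignores changes once dead.
; OnDamage stops regeneration, subtracts damage and reports death, or schedules regeneration after a delay if allowed.
; Regeneration uses timers by function name: a delayed StartRegeneration starts a looping RegenHealth.
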(fn `ChangeHealth`
  (params (Delta :type "Float (double-precision)"))
  ;[1 1 1] If not already dead
  (if (not (`self.IsDead`))
    ;[1 1 1] Reduce health by delta (and clamp between 0 and max health)
    (set `self.CurrentHealth` (`KismetMathLibrary.FClamp` (+ (`self.CurrentHealth`) Delta) 0.0 (`self.MaxHealth`)))
    ;[1 1 1] Update dead after reducing health
    (`self.UpdateDead`)))

(fn `ChangeMaxHealth`
  (params (Health :type "Float (double-precision)") (FullHealth :type Boolean))
  ;[1 1 1] Check not already dead
  (if (not (`self.IsDead`))
    ;[1 1 1] Update max health
    (set `self.MaxHealth` Health)
    ;[1 1 1] If Full Health, heal actor to max health
    (if FullHealth
      (`self.ChangeHealth` (`self.MaxHealth`)))))

(fn `InitializeHealth`
  ;[1 1 1] Set health to maximum
  (set `self.CurrentHealth` (`self.MaxHealth`)))

(fn `IsFullHealth`
  (returns (IsFullHealth :type Boolean))
  ;[1 1 1] Return whether the actor is full health (health >= maximum health)
  (return (>= (`self.CurrentHealth`) (`self.MaxHealth`))))

(fn `OnDamage`
  (params (DamageAmount :type "Float (double-precision)"))
  (returns (Died :type Boolean))
  (locals (LocalDied :type Boolean :default false))
  (`|ExecutionSequence`
    (:`then_0`
      ;[1 1 1] Stop health regeneration
      (`self.StopRegeneration`))
    (:`then_1`
      ;[1 1 1] Subtract damage
      (`self.ChangeHealth` (* DamageAmount -1.0)))
    (:`then_2`
      ;[1 1 1] Check dead
      (bind _isdead (`self.UpdateDead`))
      (bind _output_get (set `local.LocalDied` _isdead))
      ;[1 1 1] If true, return value. Else start health regen and return value
      (if _output_get
        (return (`local.LocalDied`))
        (else
          ;[1 1 1] Can this actor regen health?
          (if (`self.CanRegen`)
            ;[1 1 1] Start health regen after regen delay
            (`KismetSystemLibrary.K2_SetTimer` null "StartRegeneration" (`self.RegenDelay`))
            (return (`local.LocalDied`))))))))

(fn `RegenHealth`
  ;[1 1 1] Add regen amount to current health
  (`self.ChangeHealth` (`self.RegenAmount`)))

(fn `StartRegeneration`
  (if (`self.CanRegen`)
    (`KismetSystemLibrary.K2_SetTimer` null "RegenHealth" (`self.RegenRate`) true)))

(fn `StopRegeneration`
  ;[1 1 1] Stop the start timer
  (`KismetSystemLibrary.K2_ClearTimer` null "StartRegeneration")
  ;[1 1 1] Stop the current regen
  (`KismetSystemLibrary.K2_ClearTimer` null "RegenHealth"))

(fn `UpdateDead`
  (returns (IsDead :type Boolean))
  ;[1 1 1] Check whether character is dead (health <= 0)
  (bind _output_get (set `self.IsDead` (<= (`self.CurrentHealth`) 0.0)))
  (return _output_get))