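; BP_Enemy is the data-driven 2D roguelike enemy actor, with a flipbook sprite, box collision and health, movement and shooting components.
; SetType loads its DT_EnemyTypes row and pushes stats into those parts.
; Hits damage the player and kill the enemy, or make the movement component react to enemies, tilemaps and sprites.
; It registers with the game mode on BeginPlay; death updates room count, kills and score.
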(event `self.ReceiveBeginPlay`
  ;[1 1 1] Save game mode in variable
  (`self.SetGameMode`)
  ;[1 1 1] Add 1 (this enemy) to enemies in room
  (`/Game/Roguelike2DKit/Blueprints/Game/BP_Roguelike2DGameMode.ChangeEnemiesInRoom` (`self.GameMode`) 1)
  ;[1 1 1] Set enemy variable in Movement component
  (set `/Game/Roguelike2DKit/Blueprints/Characters/Enemies/BP_EnemyMovement.Enemy` self (`self.BP_EnemyMovement`))
  ;[1 1 1] Set enemy variable in Shooting component
  (set `/Game/Roguelike2DKit/Blueprints/Characters/Enemies/BP_EnemyShooting.Enemy` self (`self.BP_EnemyShooting`)))

(event `self.ReceiveHit`
  (params (MyComp :type "PrimitiveComponent Object Reference") (Other :type "Actor Object Reference") (OtherComp :type "PrimitiveComponent Object Reference") (bSelfMoved :type Boolean) (HitLocation :type "Vector Structure") (HitNormal :type "Vector Structure") (NormalImpulse :type "Vector Structure") (Hit :type "HitResult Structure (by ref)"))
  ;[1 1 1] Handle hit on event Hit
  (`self.HandleHit` Other OtherComp HitNormal))

(event `self.ReceiveAnyDamage`
  (params (Damage :type "Float (single-precision)") (DamageType :type "DamageType Object Reference") (InstigatedBy :type "Controller Object Reference") (DamageCauser :type "Actor Object Reference"))
  ;[1 1 1] Handle damage on event AnyDamage
  (`self.HandleDamage` Damage))

(fn `Disable`
  ;[1 1 1] Disable enemy movement
  (`/Game/Roguelike2DKit/Blueprints/Characters/Enemies/BP_EnemyMovement.Disable` (`self.BP_EnemyMovement`))
  ;[1 1 1] Disable enemy shooting
  (`/Game/Roguelike2DKit/Blueprints/Characters/Enemies/BP_EnemyShooting.Disable` (`self.BP_EnemyShooting`)))

(fn `HandleDamage`
  (params (DamageAmount :type "Float (double-precision)"))
  ;[1 1 1] Handle Damage in Component
  (bind _died (`/Game/Roguelike2DKit/Blueprints/Characters/BP_HealthComponent.OnDamage` (`self.BP_HealthComponent`) DamageAmount))
  ;[1 1 1] If dead, handle death
  (if _died
    (`self.HandleDeath`)))

(fn `HandleDeath`
  (bind _gamemode (`self.GameMode`)
    (:`then`
      ;[1 1 1] Destroy enemy actor
      (`self.K2_DestroyActor`)
      (`|ExecutionSequence`
        (:`then_0`
          ;[1 1 1] Update enemy amount in room
          (`/Game/Roguelike2DKit/Blueprints/Game/BP_Roguelike2DGameMode.ChangeEnemiesInRoom` _gamemode -1))
        (:`then_1`
          ;[1 1 1] Update enemies killed
          (`/Game/Roguelike2DKit/Blueprints/Game/BP_Roguelike2DGameMode.ChangeEnemiesKilled` _gamemode 1))
        (:`then_2`
          ;[1 1 1] Update score
          (`/Game/Roguelike2DKit/Blueprints/Game/BP_Roguelike2DGameMode.ChangeScore` _gamemode (`self.Score`)))))
    (:`else`)))

(fn `HandleHit`
  (params (OtherActor :type "Actor Object Reference") (OtherComponent :type "ActorComponent Object Reference") (HitNormal :type "Vector Structure"))
  (`|ExecutionSequence`
    (:`then_0`
      ;[1 1 1] Check for hit Player
      (bind _asbp_player (cast `/Game/Roguelike2DKit/Blueprints/Characters/Player/BP_Player` OtherActor))
      ;[1 1 1] If hit player, deal collision damage to player and handle death
      (`GameplayStatics.ApplyDamage` _asbp_player (`self.CollisionDamage`) null self)
      (`self.HandleDeath`))
    (:`then_1`
      ;[1 1 1] Check for hit other Enemy
      (cast `/Game/Roguelike2DKit/Blueprints/Characters/Enemies/BP_Enemy` OtherActor)
      ;[1 1 1] If hit enemy, handle hit in movement (change direction)
      (`/Game/Roguelike2DKit/Blueprints/Characters/Enemies/BP_EnemyMovement.HitEnemy` (`self.BP_EnemyMovement`)))
    (:`then_2`
      ;[1 1 1] Check for hit tilemap or obstacles
      (cast `PaperTileMapComponent` OtherComponent)
      ;[1 1 1] If hit, handle hit in movement (change direction)
      (`/Game/Roguelike2DKit/Blueprints/Characters/Enemies/BP_EnemyMovement.HitWall` (`self.BP_EnemyMovement`) HitNormal :!label _label))
    (:`then_3`
      (cast `PaperSpriteComponent` OtherComponent)
      (goto _label))))

(fn `LoadOptionsFromDataTable`
  (bind _returnvalue (`|GetEnumeratorNameAsString` (`self.Type`)))
  ;[1 1 1] Load options from DataTable using Enemy Type value
  (bind _returnvalue_2 (`|GetDataTableRow` "/Game/Roguelike2DKit/Blueprints/Characters/Enemies/DT_EnemyTypes.DT_EnemyTypes" (`KismetStringLibrary.Conv_StringToName` _returnvalue))
    (:`then`
      ;[1 1 1] Set options variable
      (set `self.Options` _returnvalue_2)
      ;[1 1 1] Update enemy values using options
      (`self.UpdateOptions`))
    (:`RowNotFound`
      ;[1 1 1] Print error when row is not found
      (`KismetSystemLibrary.PrintString` (`KismetStringLibrary.Concat_StrStr` "DataTable Row does not Exist for value:" _returnvalue) true true (struct :`R` 1.0 :`A` 1.0)))))

(fn `SetGameMode`
  ;[1 1 1] Gets and casts the game mode
  (bind _asbp_roguelike_2dgame_mode (cast `/Game/Roguelike2DKit/Blueprints/Game/BP_Roguelike2DGameMode` (`GameplayStatics.GetGameMode`))
    (:`then`
      ;[1 1 1] Save in variable on successfull cast
      (set `self.GameMode` _asbp_roguelike_2dgame_mode))
    (:`CastFailed`
      ;[1 1 1] Else, print an error
      (`KismetSystemLibrary.PrintString` "Invalid GameMode detected in Enemy"))))

(fn `SetType`
  (params (Type :type "/Game/Roguelike2DKit/Blueprints/Characters/Enemies/Types/ENUM_EnemyTypes Enum" :default "NewEnumerator0"))
  ;[1 1 1] Set type
  (set `self.Type` Type)
  ;[1 1 1] Load and update options based on type
  (`self.LoadOptionsFromDataTable`))

(fn `UpdateBasicOptions`
  (params (BasicOption :type "/Game/Roguelike2DKit/Blueprints/Characters/Enemies/Options/STR_BasicOptions Structure"))
  (`|ExecutionSequence`
    (:`then_0`
      ;[1 1 1] Update the sprite
      (`self.UpdateSprite` BasicOption_AliveFlipbook_6_0CD1F7274FB441BD7B549AAF9CC1B4DE BasicOption_FlipbookLocation_33_C6EA1F1A44819219AD6AC1821575DE78 BasicOption_FlipbookRotation_29_A59CEEED4D35B0349B4240B8DC34EA7F BasicOption_FlipbookScale_25_7B3B2A6A492320BFE2C756BCDC15FBC7))
    (:`then_1`
      ;[1 1 1] Update collision size
      (`self.UpdateCollisionSize` BasicOption_BoxCollisionExtent_31_AD5E4B8D4C429EC3DB6716BB8863872E))
    (:`then_2`
      ;[1 1 1] Update collision damage
      (set `self.CollisionDamage` BasicOption_CollisionDamage_24_36109E1E4414E988742AE18C298E2CFC))
    (:`then_3`
      ;[1 1 1] Update the score
      (set `self.Score` BasicOption_Score_8_49BF42D34402080F31E753BF35D5E26B))))

(fn `UpdateCollisionSize`
  (params (CollisionBoxExtent :type "Vector Structure"))
  ;[1 1 1] Update the collision box extent
  (`BoxComponent.SetBoxExtent` (`self.Box`) CollisionBoxExtent true))

(fn `UpdateHealthOptions`
  (params (HealthOptions :type "/Game/Roguelike2DKit/Blueprints/Characters/Enemies/Options/STR_HealthOptions Structure"))
  (bind _bp_healthcomponent (`self.BP_HealthComponent`))
  (`|ExecutionSequence`
    (:`then_0`
      ;[1 1 1] Update maximum health
      (`/Game/Roguelike2DKit/Blueprints/Characters/BP_HealthComponent.ChangeMaxHealth` _bp_healthcomponent HealthOptions_MaxHealth_30_E8A6374048526A7EB6F629A37A2BC0D2 true))
    (:`then_1`
      ;[1 1 1] Set Health Regen options
      (set `/Game/Roguelike2DKit/Blueprints/Characters/BP_HealthComponent.CanRegen` HealthOptions_CanRegen_32_291968814925303DB84CBF8E89A07736 _bp_healthcomponent))
    (:`then_2`
      (set `/Game/Roguelike2DKit/Blueprints/Characters/BP_HealthComponent.RegenRate` HealthOptions_RegenRate_40_1222D98341C91A60BDFD859E479386AC _bp_healthcomponent))
    (:`then_3`
      (set `/Game/Roguelike2DKit/Blueprints/Characters/BP_HealthComponent.RegenAmount` HealthOptions_RegenAmount_41_3DA78767425CC8E15C18D7B1375A5DE4 _bp_healthcomponent))
    (:`then_4`
      (set `/Game/Roguelike2DKit/Blueprints/Characters/BP_HealthComponent.RegenDelay` HealthOptions_RegenDelay_42_B12561924E011175640D77BA8E928309 _bp_healthcomponent))))

(fn `UpdateMovementOptions`
  (params (MovementOptions :type "/Game/Roguelike2DKit/Blueprints/Characters/Enemies/Options/STR_MovementOptions Structure"))
  (`|ExecutionSequence`
    (:`then_0`
      ;[1 1 1] Call update options of movement component
      (`/Game/Roguelike2DKit/Blueprints/Characters/Enemies/BP_EnemyMovement.UpdateOptions` (`self.BP_EnemyMovement`) MovementOptions_Type_9_8E7D4F640D4EF3C9A362EEB1EB2D74D8 MovementOptions_WorldOffsetSpeed_19_BCFC29A0184C2AE11FC781B2C5F5CEB3))
    (:`then_1`
      ;[1 1 1] Update FloatingPawn speed (for Chase AI)
      (set `FloatingPawnMovement.MaxSpeed` MovementOptions_FloatingPawnSpeed_18_9D1BCA1145E29CC3590980B2B2BFBFFA (`self.FloatingPawnMovement`)))))

(fn `UpdateOptions`
  (bind (_options_type _options_basicoptions _options_healthoptions _options_movementoptions _options_shootingoptions) (break `/Game/Roguelike2DKit/Blueprints/Characters/Enemies/Options/STR_EnemyOptions` (`self.Options`)))
  (`|ExecutionSequence`
    (:`then_0`
      ;[1 1 1] Update the basic options
      (`self.UpdateBasicOptions` _options_basicoptions))
    (:`then_1`
      ;[1 1 1] Update the health options
      (`self.UpdateHealthOptions` _options_healthoptions))
    (:`then_2`
      ;[1 1 1] Update the movement options
      (`self.UpdateMovementOptions` _options_movementoptions))
    (:`then_3`
      ;[1 1 1] Update the shooting options
      (`self.UpdateShootingOptions` _options_shootingoptions))))

(fn `UpdateShootingOptions`
  (params (ShootingOptions :type "/Game/Roguelike2DKit/Blueprints/Characters/Enemies/Options/STR_ShootingOptions Structure"))
  ;[1 1 1] Call update options of shooting component
  (`/Game/Roguelike2DKit/Blueprints/Characters/Enemies/BP_EnemyShooting.UpdateOptions` (`self.BP_EnemyShooting`) `ShootingOptions_Fires?_10_786EDCEE4A397E6D6D1F139F77AE9E45` ShootingOptions_FireDirections_11_DA2DADD4C241EAE3E579DAAD22A7E8B2 ShootingOptions_ProjectileScale_20_8A6182B44E10949B8597BF8FB4965265 ShootingOptions_ProjectileDamage_17_63172D304031180A42D2D0A0FC1B92BD ShootingOptions_FireDelay_13_6EF016FC8F494B0913E70ABD365FEAC2))

(fn `UpdateSprite`
  (params (Flipbook :type "PaperFlipbook Object Reference") (Location :type "Vector Structure") (Rotation :type "Rotator Structure") (Scale :type "Vector Structure"))
  (`|ExecutionSequence`
    (:`then_0`
      ;[1 1 1] Set new Flipbook
      (`PaperFlipbookComponent.SetFlipbook` (`self.Sprite`) Flipbook))
    (:`then_1`
      ;[1 1 1] Set new flipbook location
      (`SceneComponent.K2_SetRelativeLocation` (`self.Sprite`) Location false true))
    (:`then_2`
      ;[1 1 1] Set new Flipbook rotation
      (`SceneComponent.K2_SetRelativeRotation` (`self.Sprite`) Rotation false false))
    (:`then_3`
      ;[1 1 1] Set new Flipbook scale
      (`SceneComponent.SetWorldScale3D` (`self.Sprite`) Scale))))

(fn `UserConstructionScript`)