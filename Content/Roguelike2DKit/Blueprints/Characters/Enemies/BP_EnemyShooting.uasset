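; BP_EnemyShooting handles timed projectile attacks for its owning enemy.
; UpdateOptions applies settings and calls Initialize only when shooting is allowed, starting a looping timer on FireProjectile that Disable clears.
; Each shot spawns a BP_EnemyProjectile at the enemy per direction from GetProjectileDirections, passing it damage and direction.
; The Type enum selects forward, four diagonals, four cardinals, or toward the player's current position.
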(fn `Disable`
  ;[1 1 1] Disables the shooting by clearing the looping timer
  (`KismetSystemLibrary.K2_ClearTimer` null "FireProjectile"))

(fn `FireProjectile`
  ;[1 1 1] For each projectile direction, spawn an Enemy Projectile
  (for _array_element (`self.GetProjectileDirections`)
    (bind _returnvalue (`|SpawnActorFromClass` "/Game/Roguelike2DKit/Blueprints/Projectiles/BP_EnemyProjectile.BP_EnemyProjectile_C" (`KismetMathLibrary.MakeTransform` (`Actor.K2_GetActorLocation` (`self.Enemy`)) (struct) (`self.ProjectileScale`)) "AdjustIfPossibleButAlwaysSpawn" "OverrideRootScale" null null))
    (`/Engine/EditorBlueprintResources/StandardMacros.IsValid` _returnvalue
      (:`Is Valid`
        (`|ExecutionSequence`
          (:`then_0`
            ;[1 1 1] Set the projectile damage
            (set `/Game/Roguelike2DKit/Blueprints/Projectiles/BP_EnemyProjectile.Damage` (`self.ProjectileDamage`) _returnvalue))
          (:`then_1`
            ;[1 1 1] Set the projectile direction
            (`/Game/Roguelike2DKit/Blueprints/Projectiles/BP_EnemyProjectile.SetDirection` _returnvalue _array_element)))))))

(fn `GetProjectileDirections`
  (returns (Directions :type "Array of Vector Structure"))
  (locals (Result :type "Array of Vector Structure"))
  (switch `/Game/Roguelike2DKit/Blueprints/Characters/Enemies/Types/ENUM_ShootingTypes` (`self.Type`)
    (:`NewEnumerator1`
      ;[1 1 1] Return enemy forward vector
      (set `local.Result` (`|MakeArray` (`Actor.GetActorForwardVector` (`self.Enemy`)))))
    (:`NewEnumerator3`
      ;[1 1 1] Return all diagonal directions (NE, NW, SE, SW)
      (set `local.Result` (`|MakeArray` (`/Game/Roguelike2DKit/Blueprints/Directions/BP_DirectionFunctionLibrary.DirectionToVector` "NewEnumerator5") (`/Game/Roguelike2DKit/Blueprints/Directions/BP_DirectionFunctionLibrary.DirectionToVector` "NewEnumerator6") (`/Game/Roguelike2DKit/Blueprints/Directions/BP_DirectionFunctionLibrary.DirectionToVector` "NewEnumerator7") (`/Game/Roguelike2DKit/Blueprints/Directions/BP_DirectionFunctionLibrary.DirectionToVector` "NewEnumerator8"))))
    (:`NewEnumerator2`
      ;[1 1 1] Return all straight directions (N, S, E, W)
      (set `local.Result` (`|MakeArray` (`/Game/Roguelike2DKit/Blueprints/Directions/BP_DirectionFunctionLibrary.DirectionToVector` "NewEnumerator0") (`/Game/Roguelike2DKit/Blueprints/Directions/BP_DirectionFunctionLibrary.DirectionToVector` "NewEnumerator1") (`/Game/Roguelike2DKit/Blueprints/Directions/BP_DirectionFunctionLibrary.DirectionToVector` "NewEnumerator2") (`/Game/Roguelike2DKit/Blueprints/Directions/BP_DirectionFunctionLibrary.DirectionToVector` "NewEnumerator3"))))
    (:`NewEnumerator7`
      ;[1 1 1] Return the direction of the player, calculated using player and enemy position
      (set `local.Result` (`|MakeArray` (`KismetMathLibrary.Normal` (- (`Actor.K2_GetActorLocation` (`GameplayStatics.GetPlayerPawn` 0)) (`Actor.K2_GetActorLocation` (`self.Enemy`))))))))
  ;[1 1 1] Return the result
  (return (`local.Result`)))

(fn `Initialize`
  ;[1 1 1] Check can shoot
  (if (`self.CanShoot`)
    ;[1 1 1] If can shoot, call FireProjectile looping with FireDelay time in between
    (`KismetSystemLibrary.K2_SetTimer` null "FireProjectile" (`self.FireDelay`) true)))

(fn `UpdateOptions`
  (params (CanShoot :type Boolean) (Type :type "/Game/Roguelike2DKit/Blueprints/Characters/Enemies/Types/ENUM_ShootingTypes Enum" :default "NewEnumerator1") (ProjectileScale :type "Vector Structure") (ProjectileDamage :type "Float (double-precision)") (FireDelay :type "Float (double-precision)"))
  ;[1 1 1] Only set value if enemy can shoot
  (if CanShoot
    (`|ExecutionSequence`
      (:`then_0`
        ;[1 1 1] Set shooting options
        (set `self.CanShoot` CanShoot))
      (:`then_1`
        (set `self.Type` Type))
      (:`then_2`
        (set `self.ProjectileScale` ProjectileScale))
      (:`then_3`
        (set `self.ProjectileDamage` ProjectileDamage))
      (:`then_4`
        (set `self.FireDelay` FireDelay))
      (:`then_5`
        ;[1 1 1] Initialize shooting
        (`self.Initialize`)))))