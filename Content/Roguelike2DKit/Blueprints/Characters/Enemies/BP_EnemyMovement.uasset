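; Moves a roguelike enemy according to a movement type: static, axis patrol, random, bouncing or player chase.
; UpdateOptions sets type and speed, then picks a starting direction and rotates the enemy to face it.
; Tick sweeps the enemy forward by world offset, or feeds movement input toward the player when chasing, until disabled.
; Enemy and wall hits reverse, re-randomise or reflect the direction, using the hit normal for diagonal bounces.
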(event `HitEnemy`
  ;[1 1 1] On hit enemy or hit wall, change direction
  (`self.ChangeDirection` (stale `HitWall` HitNormal) :!label _label))

(event `HitWall`
  (params (HitNormal :type "Vector Structure"))
  ;[1 1 1] On hit enemy or hit wall, change direction
  (goto _label))

(event `self.ReceiveTick`
  (params (DeltaSeconds :type "Float (single-precision)"))
  ;[1 1 1] Check movement disabled
  (if (not (`self.Disabled`))
    ;[1 1 1] Check if type is Chase Player
    (if (`|EnumEquality` (`self.Type`) "NewEnumerator7")
      ;[1 1 1] Determine the chase direction (to the player) and add input
      (`Pawn.AddMovementInput` (`self.Enemy`) (`self.GetChaseDirection`) 1.0 false)
      (else
        ;[1 1 1] Else, move enemy in forward direction with movement speed
        (`Actor.K2_AddActorWorldOffset` (`self.Enemy`) (* (`Actor.GetActorForwardVector` (`self.Enemy`)) (`self.WorldOffsetSpeed`)) true false)))))

(fn `ChangeDirection`
  (params (`Hit Normal` :type "Vector Structure"))
  ;[1 1 1] Change and set direction based on current direction and movement type
  (set `self.Direction` (select `/Game/Roguelike2DKit/Blueprints/Characters/Enemies/Types/ENUM_MovementTypes` (`self.Type`) :`NewEnumerator0` "NewEnumerator4" :`NewEnumerator5` (`/Game/Roguelike2DKit/Blueprints/Directions/BP_DirectionFunctionLibrary.InverseDirection` (`self.Direction`)) :`NewEnumerator6` (`/Game/Roguelike2DKit/Blueprints/Directions/BP_DirectionFunctionLibrary.InverseDirection` (`self.Direction`)) :`NewEnumerator1` (`/Game/Roguelike2DKit/Blueprints/Directions/BP_DirectionFunctionLibrary.RandomStraightDirection`) :`NewEnumerator3` (`/Game/Roguelike2DKit/Blueprints/Directions/BP_DirectionFunctionLibrary.RandomDiagonalDirection`) :`NewEnumerator2` (`/Game/Roguelike2DKit/Blueprints/Directions/BP_DirectionFunctionLibrary.RandomMultiDirection`) :`NewEnumerator9` (`/Game/Roguelike2DKit/Blueprints/Directions/BP_DirectionFunctionLibrary.InverseDirection` (`self.Direction`)) :`NewEnumerator8` (`/Game/Roguelike2DKit/Blueprints/Directions/BP_DirectionFunctionLibrary.DiagonalBounceDirection` (`self.Direction`) (`KismetMathLibrary.NearlyEqual_FloatFloat` (`KismetMathLibrary.Abs` `Hit Normal_X`) 1.0 0.1)) :`NewEnumerator7` "NewEnumerator4"))
  ;[1 1 1] Update enemy rotation
  (`self.UpdateRotation`))

(fn `Disable`
  ;[1 1 1] Disable tick movement
  (set `self.Disabled` true))

(fn `GetChaseDirection`
  (returns (ChaseDirection :type "Vector Structure"))
  (return (`KismetMathLibrary.Normal` (- (`Actor.K2_GetActorLocation` (`GameplayStatics.GetPlayerPawn` 0)) (`Actor.K2_GetActorLocation` (`self.Enemy`))))))

(fn `InitializeDirection`
  ;[1 1 1] Initialize and set direction based on movement type
  (set `self.Direction` (select `/Game/Roguelike2DKit/Blueprints/Characters/Enemies/Types/ENUM_MovementTypes` (`self.Type`) :`NewEnumerator0` "NewEnumerator4" :`NewEnumerator5` (`/Game/Roguelike2DKit/Blueprints/Directions/BP_DirectionFunctionLibrary.RandomNorthSouthDirection`) :`NewEnumerator6` (`/Game/Roguelike2DKit/Blueprints/Directions/BP_DirectionFunctionLibrary.RandomEastWestDirection`) :`NewEnumerator1` (`/Game/Roguelike2DKit/Blueprints/Directions/BP_DirectionFunctionLibrary.RandomStraightDirection`) :`NewEnumerator3` (`/Game/Roguelike2DKit/Blueprints/Directions/BP_DirectionFunctionLibrary.RandomDiagonalDirection`) :`NewEnumerator2` (`/Game/Roguelike2DKit/Blueprints/Directions/BP_DirectionFunctionLibrary.RandomMultiDirection`) :`NewEnumerator9` (`/Game/Roguelike2DKit/Blueprints/Directions/BP_DirectionFunctionLibrary.RandomStraightDirection`) :`NewEnumerator8` (`/Game/Roguelike2DKit/Blueprints/Directions/BP_DirectionFunctionLibrary.RandomDiagonalDirection`) :`NewEnumerator7` "NewEnumerator4"))
  ;[1 1 1] Update enemy rotation
  (`self.UpdateRotation`))

(fn `UpdateOptions`
  (params (Type :type "/Game/Roguelike2DKit/Blueprints/Characters/Enemies/Types/ENUM_MovementTypes Enum" :default "NewEnumerator0") (WorldOffsetSpeed :type "Float (double-precision)"))
  ;[1 1 1] Set movement type
  (set `self.Type` Type)
  ;[1 1 1] Set movement speed
  (set `self.WorldOffsetSpeed` WorldOffsetSpeed)
  ;[1 1 1] Initialize direction based on options
  (`self.InitializeDirection`))

(fn `UpdateRotation`
  ;[1 1 1] Set rotation to forward vector of direction
  (`Actor.K2_SetActorRotation` (`self.Enemy`) (`KismetMathLibrary.MakeRotationFromAxes` (`/Game/Roguelike2DKit/Blueprints/Directions/BP_DirectionFunctionLibrary.DirectionToVector` (`self.Direction`))) false))