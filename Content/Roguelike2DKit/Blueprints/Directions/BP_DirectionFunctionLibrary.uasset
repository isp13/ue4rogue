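; Blueprint function library of helpers for the eight-way direction enum in the Roguelike 2D Kit.
; Random pickers return straight, diagonal, any, North/South or East/West directions, relying on the enum's numeric order for the ranged picks.
; Select maps give the inverse direction and diagonal bounces off side or top/bottom surfaces.
; DirectionToVector converts directions to XZ-plane vectors, with unnormalized diagonals.
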(fn `DiagonalBounceDirection`
  (params (OriginalDirection :type "/Game/Roguelike2DKit/Blueprints/Directions/ENUM_Directions Enum" :default "NewEnumerator4") (`X-Axis` :type Boolean))
  (returns (NewDirection :type "/Game/Roguelike2DKit/Blueprints/Directions/ENUM_Directions Enum"))
  (locals (Result :type "/Game/Roguelike2DKit/Blueprints/Directions/ENUM_Directions Enum"))
  (return (select `bool` `X-Axis` :`false` (select `/Game/Roguelike2DKit/Blueprints/Directions/ENUM_Directions` OriginalDirection :`NewEnumerator4` "NewEnumerator4" :`NewEnumerator0` "NewEnumerator1" :`NewEnumerator1` "NewEnumerator0" :`NewEnumerator2` "NewEnumerator3" :`NewEnumerator3` "NewEnumerator2" :`NewEnumerator5` "NewEnumerator7" :`NewEnumerator6` "NewEnumerator8" :`NewEnumerator7` "NewEnumerator5" :`NewEnumerator8` "NewEnumerator6" :!type "/Game/Roguelike2DKit/Blueprints/Directions/ENUM_Directions Enum") :`true` (select `/Game/Roguelike2DKit/Blueprints/Directions/ENUM_Directions` OriginalDirection :`NewEnumerator4` "NewEnumerator4" :`NewEnumerator0` "NewEnumerator1" :`NewEnumerator1` "NewEnumerator0" :`NewEnumerator2` "NewEnumerator3" :`NewEnumerator3` "NewEnumerator2" :`NewEnumerator5` "NewEnumerator6" :`NewEnumerator6` "NewEnumerator5" :`NewEnumerator7` "NewEnumerator8" :`NewEnumerator8` "NewEnumerator7" :!type "/Game/Roguelike2DKit/Blueprints/Directions/ENUM_Directions Enum"))))

(fn `DirectionToVector`
  (params (Direction :type "/Game/Roguelike2DKit/Blueprints/Directions/ENUM_Directions Enum" :default "NewEnumerator4"))
  (returns (Vector :type "Vector Structure"))
  (return (select `/Game/Roguelike2DKit/Blueprints/Directions/ENUM_Directions` Direction :`NewEnumerator0` (0.0 0.0 1.0) :`NewEnumerator1` (0.0 0.0 -1.0) :`NewEnumerator2` (1.0 0.0 0.0) :`NewEnumerator3` (-1.0 0.0 0.0) :`NewEnumerator5` (1.0 0.0 1.0) :`NewEnumerator6` (-1.0 0.0 1.0) :`NewEnumerator7` (1.0 0.0 -1.0) :`NewEnumerator8` (-1.0 0.0 -1.0) :!type "Vector Structure")))

(fn `InverseDirection`
  (params (OriginalDirection :type "/Game/Roguelike2DKit/Blueprints/Directions/ENUM_Directions Enum" :default "NewEnumerator4"))
  (returns (InverseDirection :type "/Game/Roguelike2DKit/Blueprints/Directions/ENUM_Directions Enum"))
  (return (select `/Game/Roguelike2DKit/Blueprints/Directions/ENUM_Directions` OriginalDirection :`NewEnumerator4` "NewEnumerator4" :`NewEnumerator0` "NewEnumerator1" :`NewEnumerator1` "NewEnumerator0" :`NewEnumerator2` "NewEnumerator3" :`NewEnumerator3` "NewEnumerator2" :`NewEnumerator5` "NewEnumerator8" :`NewEnumerator6` "NewEnumerator7" :`NewEnumerator7` "NewEnumerator6" :`NewEnumerator8` "NewEnumerator5" :!type "/Game/Roguelike2DKit/Blueprints/Directions/ENUM_Directions Enum")))

(fn `RandomDiagonalDirection`
  (returns (Direction :type "/Game/Roguelike2DKit/Blueprints/Directions/ENUM_Directions Enum"))
  (return (cast `/Game/Roguelike2DKit/Blueprints/Directions/ENUM_Directions` (`KismetMathLibrary.Conv_IntToByte` (`KismetMathLibrary.RandomIntegerInRange` 5 8)))))

(fn `RandomEastWestDirection`
  (returns (Direction :type "/Game/Roguelike2DKit/Blueprints/Directions/ENUM_Directions Enum"))
  (return (select `bool` (`KismetMathLibrary.RandomBool`) :`false` "NewEnumerator2" :`true` "NewEnumerator3" :!type "/Game/Roguelike2DKit/Blueprints/Directions/ENUM_Directions Enum")))

(fn `RandomMultiDirection`
  (returns (Direction :type "/Game/Roguelike2DKit/Blueprints/Directions/ENUM_Directions Enum"))
  (return (cast `/Game/Roguelike2DKit/Blueprints/Directions/ENUM_Directions` (`KismetMathLibrary.Conv_IntToByte` (`KismetMathLibrary.RandomIntegerInRange` 1 8)))))

(fn `RandomNorthSouthDirection`
  (returns (Direction :type "/Game/Roguelike2DKit/Blueprints/Directions/ENUM_Directions Enum"))
  (return (select `bool` (`KismetMathLibrary.RandomBool`) :`false` "NewEnumerator0" :`true` "NewEnumerator1" :!type "/Game/Roguelike2DKit/Blueprints/Directions/ENUM_Directions Enum")))

(fn `RandomStraightDirection`
  (returns (Direction :type "/Game/Roguelike2DKit/Blueprints/Directions/ENUM_Directions Enum"))
  (return (cast `/Game/Roguelike2DKit/Blueprints/Directions/ENUM_Directions` (`KismetMathLibrary.Conv_IntToByte` (`KismetMathLibrary.RandomIntegerInRange` 1 4)))))