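; BP_Chest is a locked chest terrain actor that a player opens by touching it while holding a key.
; On box overlap with BP_Player, it consumes one key, destroys itself and spawns a random pickup at its transform.
; RandomPickupClass picks the pickup by shuffling ItemsToSpawn and taking the first entry, printing an error if the list is empty.
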(event `self.Box.OnComponentBeginOverlap`
  (params (OverlappedComponent :type "PrimitiveComponent Object Reference") (OtherActor :type "Actor Object Reference") (OtherComp :type "PrimitiveComponent Object Reference") (OtherBodyIndex :type Integer) (bFromSweep :type Boolean) (SweepResult :type "HitResult Structure (by ref)"))
  ;[1 1 1] On overlap player, check if player has keys
  (bind _asbp_player (cast `/Game/Roguelike2DKit/Blueprints/Characters/Player/BP_Player` OtherActor))
  (if (`/Game/Roguelike2DKit/Blueprints/Characters/Player/BP_Player.HasKeys` _asbp_player)
    ;[1 1 1] Reduce number of keys by 1
    (`/Game/Roguelike2DKit/Blueprints/Characters/Player/BP_Player.AddKeys` _asbp_player -1)
    ;[1 1 1] Destroy chest
    (`self.K2_DestroyActor`)
    ;[1 1 1] Spawn random pickup
    (`|SpawnActorFromClass` (`self.RandomPickupClass`) (`self.GetTransform`) "Undefined" "OverrideRootScale" null null)))

(fn `RandomPickupClass`
  (returns (PickupClass :type "/Game/Roguelike2DKit/Blueprints/Pickups/BP_BasePickup Class Reference"))
  (bind _itemstospawn (`self.ItemsToSpawn`))
  ;[1 1 1] Check if there are item classes to spawn
  (if (!= (`KismetArrayLibrary.Array_Length` (`self.ItemsToSpawn`)) 0)
    ;[1 1 1] If there are classes, return a random pickup class
    (`KismetArrayLibrary.Array_Shuffle` _itemstospawn)
    (return (`|GetArrayItem` _itemstospawn))
    (else
      ;[1 1 1] Else, print an error
      (`KismetSystemLibrary.PrintString` "Empty ItemsToSpawn list  in Chest"))))

(fn `UserConstructionScript`
  (`parent.UserConstructionScript`))