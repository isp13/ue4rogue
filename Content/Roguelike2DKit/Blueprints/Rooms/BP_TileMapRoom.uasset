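; Roguelike room that builds itself from a randomly picked tile map and has a lockable door.
; On Create, it reads tile user data as spawn markers, blanks the marker layer, spawns enemies, pickups, chests and crates, then teleports the player to the start.
; Player overlap with the trigger marks it finished and calls GameMode CleanupRoom.
; Destroy clears spawn points and removes every spawnable actor in the world, found by interface.
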(event `/Game/Roguelike2DKit/Blueprints/Rooms/BP_iRoom.Create`
  ;[1 1 1] Create a new room on event Create
  (`self.CreateRoom`))

(event `/Game/Roguelike2DKit/Blueprints/Rooms/BP_iRoom.Destroy`
  ;[1 1 1] Destroy Spawnables and clear SpawnPoints on event Destroy
  (`self.DestroySpawnables`)
  (`self.ClearSpawnPoints`))

(event `/Game/Roguelike2DKit/Blueprints/Rooms/BP_iRoom.Unlock`
  ;[1 1 1] Unlock gates on event Unlock
  (`self.UnlockGates`))

(event `/Game/Roguelike2DKit/Blueprints/Rooms/BP_iRoom.Lock`
  ;[1 1 1] Lock gates on event Lock
  (`self.LockGates`))

(event `self.Trigger.OnComponentBeginOverlap`
  (params (OverlappedComponent :type "PrimitiveComponent Object Reference") (OtherActor :type "Actor Object Reference") (OtherComp :type "PrimitiveComponent Object Reference") (OtherBodyIndex :type Integer) (bFromSweep :type Boolean) (SweepResult :type "HitResult Structure (by ref)"))
  ;[1 1 1] Check room finished
  (if (not (`self.Finished`))
    ;[1 1 1] If overlapping player, set finished
    (cast `/Game/Roguelike2DKit/Blueprints/Characters/Player/BP_Player` OtherActor)
    (set `self.Finished` true)
    ;[1 1 1] Let Game Mode clean-up room
    (bind _asbp_roguelike_2dgame_mode (cast `/Game/Roguelike2DKit/Blueprints/Game/BP_Roguelike2DGameMode` (`GameplayStatics.GetGameMode`)))
    (`/Game/Roguelike2DKit/Blueprints/Game/BP_Roguelike2DGameMode.CleanupRoom` _asbp_roguelike_2dgame_mode)))

(fn `AnalyzeSetupData`
  (locals (TileMapLocation :type "/Game/Roguelike2DKit/Blueprints/Rooms/STR_TileMapLocation Structure"))
  (bind (_tilemaplocation_x _tilemaplocation_y _tilemaplocation_layer) (break `/Game/Roguelike2DKit/Blueprints/Rooms/STR_TileMapLocation` (`local.TileMapLocation`)))
  (bind _returnvalue (`TileMapBlueprintLibrary.GetTileUserData` (`PaperTileMapComponent.GetTile` (`self.Room`) _tilemaplocation_x _tilemaplocation_y _tilemaplocation_layer)))
  (bind (_isenemy _enemytype) (`self.IsEnemy` _returnvalue))
  ;[1 1 1] Loops over all tiles in Setup Room
  (bind (_mapwidth _mapheight _numlayers) (`PaperTileMapComponent.GetMapSize` (`self.Room`)))
  ;[1 1 1] Loop over layers
  (for _index (range (+ _numlayers 1))
    ;[1 1 1] Loop over Y value
    (for _index_2 (range (+ _mapwidth 1))
      ;[1 1 1] Loop over X value
      (for _index_3 (range (+ _mapheight 1))
        ;[1 1 1] Save tile location in variable
        (set `local.TileMapLocation` (make `/Game/Roguelike2DKit/Blueprints/Rooms/STR_TileMapLocation` _index_2 _index_3 _index))
        ;[1 1 1] Check if the data specifies an Enemy and which type
        (if _isenemy
          ;[1 1 1] Add Enemy Spawn point
          (`BlueprintMapLibrary.Map_Add` (`self.EnemySpawnPoints`) (`local.TileMapLocation`) _enemytype)
          (else
            ;[1 1 1] Switch on Tile User Data. Match on name to define non-enemy spawn points
            (switch `name` _returnvalue
              (:`Key`
                ;[1 1 1] Add Key Spawn point
                (`KismetArrayLibrary.Array_AddUnique` (`self.KeySpawnPoints`) (`local.TileMapLocation`)))
              (:`Chest`
                ;[1 1 1] Add Chest spawn point
                (`KismetArrayLibrary.Array_AddUnique` (`self.ChestSpawnPoints`) (`local.TileMapLocation`)))
              (:`Heart`
                ;[1 1 1] Add Health Pickup spawn point
                (`KismetArrayLibrary.Array_AddUnique` (`self.HeartSpawnPoints`) (`local.TileMapLocation`)))
              (:`Breakable`
                ;[1 1 1] Add Breakable spawn point
                (`KismetArrayLibrary.Array_AddUnique` (`self.BreakableCrateSpawnPoints`) (`local.TileMapLocation`)))
              (:`Bomb`
                ;[1 1 1] Add Bomb (pickup) spawn point
                (`KismetArrayLibrary.Array_AddUnique` (`self.BombSpawnPoints`) (`local.TileMapLocation`)))
              (:`PlayerStart`
                ;[1 1 1] Set the player start postion using the Tile Map Location converted to World location
                (set `self.PlayerStartLocation` (`self.TileMapToWorld` (`local.TileMapLocation`)))))))))))

(fn `ChooseRandomRoom`
  (bind _possiblerooms (`self.PossibleRooms`))
  (bind _output (`|GetArrayItem` _possiblerooms))
  ;[1 1 1] Get a random room
  (`KismetArrayLibrary.Array_Shuffle` _possiblerooms)
  (`/Engine/EditorBlueprintResources/StandardMacros.IsValid` _output
    (:`Is Valid`
      ;[1 1 1] Set the Room object to the random room
      (`PaperTileMapComponent.SetTileMap` (`self.Room`) _output))
    (:`Is Not Valid`
      (`KismetSystemLibrary.PrintString` "No Valid Room Found in Rooms" true true (struct :`R` 1.0 :`A` 1.0)))))

(fn `ClearSetupData`
  ;[1 1 1] Make the room editable
  (`PaperTileMapComponent.MakeTileMapEditable` (`self.Room`))
  ;[1 1 1] Loop through all tiles of the Game layer (index 0), which contains the spawn information, and reset the Tile Index to -1
  (bind (_mapwidth _mapheight) (`PaperTileMapComponent.GetMapSize` (`self.Room`)))
  (for _index (range (+ _mapheight 1))
    (for _index_2 (range (+ _mapwidth 1))
      (`PaperTileMapComponent.SetTile` (`self.Room`) _index_2 _index 0 (make `PaperTileInfo` -1)))))

(fn `ClearSpawnPoints`
  (`|ExecutionSequence`
    (:`then_0`
      (`BlueprintMapLibrary.Map_Clear` (`self.EnemySpawnPoints`)))
    (:`then_1`
      (`KismetArrayLibrary.Array_Clear` (`self.KeySpawnPoints`)))
    (:`then_2`
      (`KismetArrayLibrary.Array_Clear` (`self.ChestSpawnPoints`)))
    (:`then_3`
      (`KismetArrayLibrary.Array_Clear` (`self.HeartSpawnPoints`)))
    (:`then_4`
      (`KismetArrayLibrary.Array_Clear` (`self.BreakableCrateSpawnPoints`)))
    (:`then_5`
      (`KismetArrayLibrary.Array_Clear` (`self.BombSpawnPoints`)))))

(fn `CreateRoom`
  ;[1 1 1] Select random room
  (`self.ChooseRandomRoom`)
  ;[1 1 1] Analyze setup data
  (`self.AnalyzeSetupData`)
  ;[1 1 1] Clear setup data
  (`self.ClearSetupData`)
  ;[1 1 1] Spawn elements in room
  (`self.SpawnElements`)
  ;[1 1 1] Move the player to the start location
  (`self.PositionPlayer` (`self.PlayerStartLocation`)))

(fn `DestroySpawnables`
  ;[1 1 1] Loop over all Spawnable actors
  (bind _outactors (`GameplayStatics.GetAllActorsWithInterface` "/Game/Roguelike2DKit/Blueprints/BP_iSpawnable.BP_iSpawnable_C"))
  (bind (_arrayindex _arrayelement) (`/Engine/EditorBlueprintResources/StandardMacros.ReverseForEachLoop` _outactors)
    (:`LoopBody`
      ;[1 1 1] Destroy each valid Spawnable
      (`/Engine/EditorBlueprintResources/StandardMacros.IsValid` _arrayelement
        (:`Is Valid`
          (`self.K2_DestroyActor` _arrayelement))))))

(fn `GetEnemyType`
  (params (EnemyType :type "/Game/Roguelike2DKit/Blueprints/Characters/Enemies/Types/ENUM_EnemyTypes Enum" :default "NewEnumerator0"))
  (returns (EnemyTypeResult :type "/Game/Roguelike2DKit/Blueprints/Characters/Enemies/Types/ENUM_EnemyTypes Enum"))
  (return (select `bool` (`|EnumEquality` EnemyType "NewEnumerator4") :`false` EnemyType :`true` (cast `/Game/Roguelike2DKit/Blueprints/Characters/Enemies/Types/ENUM_EnemyTypes` (`KismetMathLibrary.Conv_IntToByte` (`KismetMathLibrary.RandomIntegerInRange` 0 (- (enumcount `/Game/Roguelike2DKit/Blueprints/Characters/Enemies/Types/ENUM_EnemyTypes`) 2)))))))

(fn `IsEnemy`
  (params (TileUserData :type Name))
  (returns (IsEnemy :type Boolean) (EnemyType :type "/Game/Roguelike2DKit/Blueprints/Characters/Enemies/Types/ENUM_EnemyTypes Enum"))
  (locals (IsEnemyLocal :type Boolean) (EnemyTypeLocal :type "/Game/Roguelike2DKit/Blueprints/Characters/Enemies/Types/ENUM_EnemyTypes Enum" :default "NewEnumerator0"))
  ;[1 1 1] Returns true if the Tile User Data matches an EnemyTypes enum entry. Else returns false
  (bind _enumvalue (foreach `/Game/Roguelike2DKit/Blueprints/Characters/Enemies/Types/ENUM_EnemyTypes`)
    (:`LoopBody`
      (if (== TileUserData (`KismetStringLibrary.Conv_StringToName` (`|GetEnumeratorNameAsString` _enumvalue)))
        (set `local.IsEnemyLocal` true)
        (set `local.EnemyTypeLocal` _enumvalue)
        (return (`local.IsEnemyLocal`) (`local.EnemyTypeLocal`))))
    (:`then`
      (return (`local.IsEnemyLocal`) (`local.EnemyTypeLocal`)))))

(fn `LockGates`
  (bind _door (`self.Door`))
  ;[1 1 1] Change sprite to locked door
  (`PaperSpriteComponent.SetSprite` _door (`self.LockedDoorSprite`))
  ;[1 1 1] Enable blocking door
  (`PrimitiveComponent.SetCollisionProfileName` _door "BlockAllDynamic")
  ;[1 1 1] Reset the Finished variable
  (set `self.Finished` false))

(fn `PositionPlayer`
  (params (Position :type "Vector Structure"))
  (`self.K2_SetActorLocation` (`GameplayStatics.GetPlayerPawn` 0) Position false true))

(fn `SpawnActorsFromTileMapLocations`
  (params (TileMapLocations :type "Array of /Game/Roguelike2DKit/Blueprints/Rooms/STR_TileMapLocation Structure") (ClassToSpawn :type "Actor Class Reference"))
  ;[1 1 1] Loop over Tile Map locations and convert to world location
  (for _array_element TileMapLocations
    ;[1 1 1] Spawn actor of ClassToSpawn for location
    (`|SpawnActorFromClass` ClassToSpawn (`KismetMathLibrary.MakeTransform` (`self.TileMapToWorld` _array_element)) "Undefined" "OverrideRootScale" null null)))

(fn `SpawnElements`
  (`|ExecutionSequence`
    (:`then_0`
      ;[1 1 1] Spawn enemies
      (`self.SpawnEnemies`))
    (:`then_1`
      ;[1 1 1] Spawn chests
      (`self.SpawnActorsFromTileMapLocations` (`self.ChestSpawnPoints`) "/Game/Roguelike2DKit/Blueprints/Terrain/BP_Chest.BP_Chest_C"))
    (:`then_2`
      ;[1 1 1] Spawn key pickups
      (`self.SpawnActorsFromTileMapLocations` (`self.KeySpawnPoints`) "/Game/Roguelike2DKit/Blueprints/Pickups/BP_KeyPickup.BP_KeyPickup_C"))
    (:`then_3`
      ;[1 1 1] Spawn health pickups
      (`self.SpawnActorsFromTileMapLocations` (`self.HeartSpawnPoints`) "/Game/Roguelike2DKit/Blueprints/Pickups/BP_HealthPickup.BP_HealthPickup_C"))
    (:`then_4`
      ;[1 1 1] Spawn bomb pickups
      (`self.SpawnActorsFromTileMapLocations` (`self.BombSpawnPoints`) "/Game/Roguelike2DKit/Blueprints/Pickups/BP_BombPickup.BP_BombPickup_C"))
    (:`then_5`
      ;[1 1 1] Spawn breakable crates
      (`self.SpawnActorsFromTileMapLocations` (`self.BreakableCrateSpawnPoints`) "/Game/Roguelike2DKit/Blueprints/Terrain/BP_BreakableCrate.BP_BreakableCrate_C"))))

(fn `SpawnEnemies`
  (locals (SpawnedEnemy :type "/Game/Roguelike2DKit/Blueprints/Characters/Enemies/BP_Enemy Object Reference"))
  (bind _enemyspawnpoints (`self.EnemySpawnPoints`))
  ;[1 1 1] Loop over enemy spawn points
  (bind _keys (`BlueprintMapLibrary.Map_Keys` _enemyspawnpoints))
  (for (_array_element _array_index) _keys
    (`|ExecutionSequence`
      (:`then_0`
        ;[1 1 1] Spawn enemy actor on location
        (bind _returnvalue (`|SpawnActorFromClass` "/Game/Roguelike2DKit/Blueprints/Characters/Enemies/BP_Enemy.BP_Enemy_C" (`KismetMathLibrary.MakeTransform` (`self.TileMapToWorld` _array_element)) "Undefined" "OverrideRootScale" null null))
        (set `local.SpawnedEnemy` _returnvalue))
      (:`then_1`
        ;[1 1 1] Set enemy type
        (`/Engine/EditorBlueprintResources/StandardMacros.IsValid` (`local.SpawnedEnemy`)
          (:`Is Valid`
            (bind _values (`BlueprintMapLibrary.Map_Values` _enemyspawnpoints))
            (`/Game/Roguelike2DKit/Blueprints/Characters/Enemies/BP_Enemy.SetType` (`local.SpawnedEnemy`) (`self.GetEnemyType` (`|GetArrayItem` _values _array_index)))))))))

(fn `TileMapToWorld`
  (params (TileMapLocation :type "/Game/Roguelike2DKit/Blueprints/Rooms/STR_TileMapLocation Structure"))
  (returns (WorldLocation :type "Vector Structure"))
  (bind _room (`self.Room`))
  (bind _tilemap (`PaperTileMapComponent.TileMap` _room))
  ;[1 1 1] Negate Y value
  (bind _result (`/Engine/EditorBlueprintResources/StandardMacros.NegateInt` TileMapLocation_Y_5_999059334D93479B3F522598C6049571)
    (:`  `
      (return (+ (`SceneComponent.K2_GetComponentLocation` _room) (`KismetMathLibrary.MakeVector` (`KismetMathLibrary.Conv_IntToDouble` (* TileMapLocation_X_2_EADAED894F0F88468D8D689416047D71 (`PaperTileMap.TileWidth` _tilemap))) (`self.SpawnYValue`) (`KismetMathLibrary.Conv_IntToDouble` (* _result (`PaperTileMap.TileHeight` _tilemap)))))))))

(fn `UnlockGates`
  ;[1 1 1] Change door sprite to unlocked door
  (`PaperSpriteComponent.SetSprite` (`self.Door`) (`self.UnlockDoorSprite`))
  ;[1 1 1] Enable blocking door
  (`PrimitiveComponent.SetCollisionProfileName` (`self.Door`) "NoCollision"))

(fn `UserConstructionScript`)