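; Player controller for the Roguelike 2D Kit that owns the HUD and handles pausing and game over.
; On BeginPlay it creates BP_HUD, adds it to the viewport and sets game-only input.
; The PauseGame input shows the pause menu, pauses, and switches to cursor and UI input; UnpauseGame restores gameplay input.
; GameOver shows its menu with the same input switch, but does not pause.
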(event `self.ReceiveBeginPlay`
  ;[1 1 1] Create HUD and add to viewport
  (bind _returnvalue (`|CreateWidget` "/Game/Roguelike2DKit/Blueprints/Widgets/BP_HUD.BP_HUD_C"))
  (bind _output_get (set `self.HUD` _returnvalue))
  (`UserWidget.AddToViewport` _output_get 0)
  ;[1 1 1] Set input to Game Only
  (`WidgetBlueprintLibrary.SetInputMode_GameOnly` self))

(event `InputAction|PauseGame`
  (params (Key :type "Key Structure"))
  (:`Pressed`
    ;[1 1 1] Pause game
    (`self.PauseGame`)))

(fn `GameOver`
  (bind _hud (`self.HUD`))
  ;[1 1 1] Show Game Over menu
  (`/Game/Roguelike2DKit/Blueprints/Widgets/BP_HUD.ShowGameOverMenu` _hud)
  ;[1 1 1] Show cursor and set input UI only
  (set `self.bShowMouseCursor` true)
  (`WidgetBlueprintLibrary.SetInputMode_UIOnlyEx` self (`/Game/Roguelike2DKit/Blueprints/Widgets/BP_HUD.ReturnToMenuButton` _hud)))

(fn `PauseGame`
  (bind _hud (`self.HUD`))
  ;[1 1 1] Show pause menu
  (`/Game/Roguelike2DKit/Blueprints/Widgets/BP_HUD.ShowPauseMenu` _hud)
  ;[1 1 1] Pause game
  (`GameplayStatics.SetGamePaused` true)
  ;[1 1 1] Show cursor and set input to UI only
  (set `self.bShowMouseCursor` true)
  (`WidgetBlueprintLibrary.SetInputMode_UIOnlyEx` self (`/Game/Roguelike2DKit/Blueprints/Widgets/BP_HUD.ResumeButton` _hud)))

(fn `UnpauseGame`
  ;[1 1 1] Unpause the game
  (`GameplayStatics.SetGamePaused` false)
  ;[1 1 1] Hides cursor and set input to Game Only
  (set `self.bShowMouseCursor` false)
  (`WidgetBlueprintLibrary.SetInputMode_GameOnly` self))

(fn `UserConstructionScript`)