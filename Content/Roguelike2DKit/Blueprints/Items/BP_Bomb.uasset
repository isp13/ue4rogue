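; BP_Bomb is a timed bomb item for a 2D roguelike that explodes after a delay unless the game is over.
; On detonation it destroys breakables and applies damage to all PaperCharacters, player and enemies alike, overlapping its blast radius.
; It then plays a sound, disables collision, swaps to a scaled explosion flipbook and destroys itself when that animation's length has elapsed.
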(event `self.ReceiveBeginPlay`
  ;[1 1 1] Wait ExplosionDelay
  (`KismetSystemLibrary.Delay` (`self.ExplosionDelay`))
  ;[1 1 1] If not game over, explode
  (bind _asbp_roguelike_2dgame_mode (cast `/Game/Roguelike2DKit/Blueprints/Game/BP_Roguelike2DGameMode` (`GameplayStatics.GetGameMode`)))
  (if (not (`/Game/Roguelike2DKit/Blueprints/Game/BP_Roguelike2DGameMode.IsGameOver` _asbp_roguelike_2dgame_mode))
    (`|ExecutionSequence`
      (:`then_0`
        ;[1 1 1] Destroy Breakables
        (`self.DestroyBreakables`))
      (:`then_1`
        ;[1 1 1] Damage PaperCharacters
        (`self.DamagePaperActors`))
      (:`then_2`
        ;[1 1 1] Play sound
        (`GameplayStatics.PlaySound2D` (`self.ExplosionSound`)))
      (:`then_3`
        ;[1 1 1] Disable actor collision
        (`self.SetActorEnableCollision` false))
      (:`then_4`
        ;[1 1 1] Set explosion animation
        (`PaperFlipbookComponent.SetFlipbook` (`self.Sprite`) "/Game/Roguelike2DKit/Animations/FB_Explosion.FB_Explosion")
        (`SceneComponent.SetWorldScale3D` (`self.Sprite`) (`self.ExplosionFlipbookScale`)))
      (:`then_5`
        ;[1 1 1] After explosion animation is done, destroy actor
        (`KismetSystemLibrary.Delay` (`PaperFlipbookComponent.GetFlipbookLength` (`self.Sprite`)))
        (`self.K2_DestroyActor`)))))

(fn `DamagePaperActors`
  ;[1 1 1] Get all Paper Characters (enemies and player) inside the blast radius and loop over them
  (bind (_arrayindex _arrayelement) (`/Engine/EditorBlueprintResources/StandardMacros.ReverseForEachLoop` (`PrimitiveComponent.GetOverlappingActors` (`self.BlastRadius`) "/Script/Paper2D.PaperCharacter"))
    (:`LoopBody`
      ;[1 1 1] Apply bomb damage to the actor
      (`GameplayStatics.ApplyDamage` _arrayelement (`self.BombDamage`)))))

(fn `DestroyBreakables`
  ;[1 1 1] Get all Breakables inside the blast radius and loop over them
  (bind (_arrayindex _arrayelement) (`/Engine/EditorBlueprintResources/StandardMacros.ReverseForEachLoop` (`PrimitiveComponent.GetOverlappingActors` (`self.BlastRadius`) "/Game/Roguelike2DKit/Blueprints/Terrain/BP_BaseBreakable.BP_BaseBreakable_C"))
    (:`LoopBody`
      ;[1 1 1] Destroy the breakables
      (`self.K2_DestroyActor` _arrayelement))))

(fn `UserConstructionScript`)