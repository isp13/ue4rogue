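; Game mode for the 2D roguelike kit that runs the room loop and tracks run stats.
; On BeginPlay it finds the level's room actor, then creates and locks it; the room unlocks when its enemy count hits zero.
; CleanupRoom counts the clear, then destroys and recreates the room after a delay.
; GameOver freezes score changes, disables all enemies, saves the score through the game state and notifies the player controller.
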(event `self.ReceiveBeginPlay`
  ;[1 1 1] Find and save the room object
  (`self.FindRoom`)
  ;[1 1 1] Create a new room
  (`self.CreateRoom`))

(event `CleanupRoom`
  ;[1 1 1] Increment rooms cleared
  (`self.IncrementRoomsCleared`)
  ;[1 1 1] Destroy room after destroy delay
  (`KismetSystemLibrary.Delay` (`self.LevelDestroyDelay`))
  (`/Game/Roguelike2DKit/Blueprints/Rooms/BP_iRoom.Destroy` (`self.TileMapRoom`))
  ;[1 1 1] Create a new room
  (`self.CreateRoom`))

(fn `ChangeEnemiesInRoom`
  (params (Delta :type Integer))
  ;[1 1 1] Update enemies in room amount by delta
  (bind _output_get (set `self.EnemiesInRoom` (+ (`self.EnemiesInRoom`) Delta)))
  ;[1 1 1] If amount is 0, unlock the room
  (if (== _output_get 0)
    (`/Game/Roguelike2DKit/Blueprints/Rooms/BP_iRoom.Unlock` (`self.TileMapRoom`))))

(fn `ChangeEnemiesKilled`
  (params (Delta :type Integer))
  ;[1 1 1] Update enemies killed amount by delta
  (set `self.EnemiesKilled` (+ Delta (`self.EnemiesKilled`))))

(fn `ChangeScore`
  (params (Delta :type Integer))
  ;[1 1 1] Only if the game is not over
  (if (not (`self.IsGameOver`))
    ;[1 1 1] Update score amount by delta
    (set `self.Score` (+ Delta (`self.Score`)))))

(fn `CreateRoom`
  ;[1 1 1] Create a room and lock it
  (`/Game/Roguelike2DKit/Blueprints/Rooms/BP_iRoom.Create` (`self.TileMapRoom`))
  (`/Game/Roguelike2DKit/Blueprints/Rooms/BP_iRoom.Lock` (`self.TileMapRoom`)))

(fn `DisableEnemies`
  ;[1 1 1] Loop over all enemies
  (bind _outactors (`GameplayStatics.GetAllActorsOfClass` "/Game/Roguelike2DKit/Blueprints/Characters/Enemies/BP_Enemy.BP_Enemy_C"))
  (for _array_element _outactors
    ;[1 1 1] Disable enemy
    (`/Game/Roguelike2DKit/Blueprints/Characters/Enemies/BP_Enemy.Disable` _array_element)))

(fn `FindRoom`
  ;[1 1 1] Find all actors of the Room Class and get the first one
  (bind _outactors (`GameplayStatics.GetAllActorsOfClass` (`self.RoomClass`)))
  (bind _output (`|GetArrayItem` _outactors))
  ;[1 1 1] Save the room in a Variable or print error message
  (`/Engine/EditorBlueprintResources/StandardMacros.IsValid` _output
    (:`Is Valid`
      (set `self.TileMapRoom` _output)
      (return))
    (:`Is Not Valid`
      (`KismetSystemLibrary.PrintString` "No Valid Room found. \nPlease add one to the Map" true true (struct :`R` 1.0 :`A` 1.0)))))

(fn `GameOver`
  (`|ExecutionSequence`
    (:`then_0`
      ;[1 1 1] Set Game Over to true
      (set `self.IsGameOver` true))
    (:`then_1`
      ;[1 1 1] Play sound
      (`GameplayStatics.PlaySound2D` (`self.GameOverSound`)))
    (:`then_2`
      ;[1 1 1] Disable all enemies
      (`self.DisableEnemies`))
    (:`then_3`
      ;[1 1 1] Save high score
      (`self.SaveHighScore`))
    (:`then_4`
      ;[1 1 1] Notify game over controller (updates interface etcetera)
      (`self.GameOverPlayerController`))))

(fn `GameOverPlayerController`
  ;[1 1 1] Notify player controller with game over
  (bind _asbp_roguelike_2dplayer_controller (cast `/Game/Roguelike2DKit/Blueprints/PlayerControllers/BP_Roguelike2DPlayerController` (`GameplayStatics.GetPlayerController` 0)))
  (`/Game/Roguelike2DKit/Blueprints/PlayerControllers/BP_Roguelike2DPlayerController.GameOver` _asbp_roguelike_2dplayer_controller))

(fn `IncrementRoomsCleared`
  ;[1 1 1] Increments the rooms cleared counter by 1
  (set `self.RoomsCleared` (+ (`self.RoomsCleared`) 1)))

(fn `SaveHighScore`
  ;[1 1 1] Get Game State
  (bind _asbp_roguelike_2dgame_state (cast `/Game/Roguelike2DKit/Blueprints/Game/BP_Roguelike2DGameState` (`GameplayStatics.GetGameState`)))
  ;[1 1 1] Save achieved (high) score
  (`/Game/Roguelike2DKit/Blueprints/Game/BP_Roguelike2DGameState.SaveData` _asbp_roguelike_2dgame_state (`self.Score`)))

(fn `UserConstructionScript`)